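; Battle royale zone actor that steps through ZoneActions, waiting, then shrinking a scaled mesh via timeline lerps of radius, height and location.
; The server pre-generates random centers nested inside each previous zone, starts each step and multicasts shrinks.
; It previews the next zone with a temporary mesh and reports status changes to every ThirdPersonCharacter's zone component.
; A looping timer feeds zone radius and location to MPC_BRZone; camera post-process and sounds toggle at the boundary.
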(event `Apply Zone Prediction`
  (params (`Prediction Zone Index` :type Integer))
  (bind (_radius _height) (break `/Game/AdvancedBattleRoyaleZone/Blueprint/Structure/S_Zone_Actions` (`|GetArrayItem` (`self.Zone Actions`) `Prediction Zone Index`)))
  ;[0.2656 0.4221 1 1 100] Zone Prediction
  ;;[1 0.2604 0.2604] Zone Prediction.
  (if (`self.Show Next Zone?`)
    (bind _returnvalue (`AddComponent|NODE_AddStaticMeshComponent-0`))
    (bind _output_get (set `self.Prediction Zone Mesh` _returnvalue))
    (`PrimitiveComponent.SetMaterial` _output_get 0 (`self.Zone Prediction Material`))
    (`SceneComponent.SetRelativeScale3D` _output_get (`KismetMathLibrary.MakeVector` _radius _radius _height))
    (`SceneComponent.K2_SetRelativeLocation` _output_get (`|GetArrayItem` (`self.Zone Locations`) `Prediction Zone Index`) false false)))

(event `Remove Zone Prediction`
  (bind _prediction_zone_mesh (`self.Prediction Zone Mesh`))
  ;[0.2656 0.4221 1 1 100] Zone Prediction
  ;;[1 0.5622 0.2543] Remove Zone Prediction. This Event should be called only from client
  (`/Engine/EditorBlueprintResources/StandardMacros.IsValid` _prediction_zone_mesh
    (:`Is Valid`
      (`ActorComponent.K2_DestroyComponent` _prediction_zone_mesh))))

(event `Set Parameter Collections`
  (bind _returnvalue_x (`KismetMathLibrary.BreakVector` (`SceneComponent.K2_GetComponentScale` (`self.SM_Zone`))))
  (bind (_returnvalue_x_2 _returnvalue_y _returnvalue_z) (`KismetMathLibrary.BreakVector` (`SceneComponent.K2_GetComponentLocation` (`self.SM_Zone`))))
  ;[0 0 0] Set Parameter Collection
  (`KismetMaterialLibrary.SetScalarParameterValue` "/Game/AdvancedBattleRoyaleZone/Material/MaterialFunctions/ParameterCollection/MPC_BRZone.MPC_BRZone" "Zone Radius" _returnvalue_x)
  (`KismetMaterialLibrary.SetVectorParameterValue` "/Game/AdvancedBattleRoyaleZone/Material/MaterialFunctions/ParameterCollection/MPC_BRZone.MPC_BRZone" "Zone Location" (make `LinearColor` _returnvalue_x_2 _returnvalue_y _returnvalue_z 1.0)))

(event `self.ReceiveBeginPlay`
  ;[0 0 0] Begin Play
  (`self.Set Parameter Collections`)
  ;;[1 1 1] Generate Locations On Server
  (`/Engine/EditorBlueprintResources/ActorMacros.Switch Has Authority`
    (:`Authority`
      (`self.Generate New Location For Zone`))
    (:`Remote`
      _))
  (`KismetSystemLibrary.K2_SetTimerDelegate` (delegate `Set Parameter Collections`) 0.025 true)
  (`KismetSystemLibrary.Delay` 3.0) ; Setup Delay (Waiting for clients to join)
  ;;[1 1 1] Generate Locations On Server
  (`/Engine/EditorBlueprintResources/ActorMacros.Switch Has Authority`
    (:`Authority`
      ;;[1 1 1] Start Zone Action
      (`self.Do Zone Action`))))

(event `Event On Zone Is Shrinking`
  (bind _current_action_index (`self.Current Action Index`))
  ;[1 0 0] Event On Zone Shrinking
  (`self.Call Players Zone Status Changed` "NewEnumerator0" true)
  (`KismetSystemLibrary.Delay` (`self.State Change Delay`))
  (`self.Shrink Zone (Multicast)` _current_action_index (+ _current_action_index 1)))

(event `Do Zone Action`
  (bind _current_action_index (`self.Current Action Index`))
  (bind _returnvalue (+ _current_action_index 1))
  (bind ((`ZoneActionDuration_16_17F540C6441BB7F5BD2D299311AD5C8D` _zoneactionduration)) (break `/Game/AdvancedBattleRoyaleZone/Blueprint/Structure/S_Zone_Actions` (`|GetArrayItem` (`self.Zone Actions`) _current_action_index)))
  ;[0 0 0] Event Do Zone Action
  (if (`KismetArrayLibrary.Array_IsValidIndex` (`self.Zone Actions`) _returnvalue)
    (`self.Apply Zone Prediction` _returnvalue)
    (`self.Call Players Zone Status Changed` "NewEnumerator0" false _zoneactionduration)
    (`KismetSystemLibrary.Delay` _zoneactionduration)
    (`self.Event On Zone Is Shrinking`)))

(event `Event On Zone Shrinking Finished`
  ;[0 0.6087 1] Event On Shrinking Finished
  (`self.Call Players Zone Status Changed` "NewEnumerator1" true)
  (`self.Remove Zone Prediction`)
  (`KismetSystemLibrary.Delay` (`self.State Change Delay`))
  (`/Engine/EditorBlueprintResources/ActorMacros.Switch Has Authority`
    (:`Authority`
      (`self.Do Zone Action`))))

(event `Shrink Zone (Multicast)`
  (params (`Current Action Index` :type Integer) (`To Action Index` :type Integer))
  (bind ((`ShrinkSpeed_11_E476FB3542AC13C9832BB1B49D5A7BC6` _shrinkspeed)) (break `/Game/AdvancedBattleRoyaleZone/Blueprint/Structure/S_Zone_Actions` (`|GetArrayItem` (`self.Zone Actions`) `To Action Index`)))
  ;[0 0 0] Prepare For Shrinking
  (if (`KismetArrayLibrary.Array_IsValidIndex` (`self.Zone Actions`) `To Action Index`)
    (`TimelineComponent.SetPlayRate` (`self.Zone Shrinking Timeline`) (/ 1.0 _shrinkspeed))
    (`self.Shrink` `Current Action Index` `To Action Index`)
    (`self.Call Players Zone Status Changed` "NewEnumerator1" false _shrinkspeed)))

(event `Shrink`
  (params (`Current Zone Index` :type Integer) (`To Action Index` :type Integer))
  (bind ((`Radius_13_BD564BF94CFDF298438BDFABA2539C44` _radius) (`Height_4_4B72F8464D046B7663EAC1856236F50E` _height)) (break `/Game/AdvancedBattleRoyaleZone/Blueprint/Structure/S_Zone_Actions` (`|GetArrayItem` (`self.Zone Actions`) `Current Zone Index`)))
  (bind ((`Radius_13_BD564BF94CFDF298438BDFABA2539C44` _radius_2) (`Height_4_4B72F8464D046B7663EAC1856236F50E` _height_2)) (break `/Game/AdvancedBattleRoyaleZone/Blueprint/Structure/S_Zone_Actions` (`|GetArrayItem` (`self.Zone Actions`) `To Action Index`)))
  ;[0 0 0] Zone Shrinking
  (bind (_direction _alpha) (`Timeline|Zone Shrinking Timeline` :`NewTime` 0.0 :!via `PlayFromStart`)
    (:`Update`
      (`self.Set Zone Transform` (`KismetMathLibrary.Lerp` _radius _radius_2 _alpha) (`KismetMathLibrary.Lerp` _height _height_2 _alpha) (`KismetMathLibrary.VLerp` (`|GetArrayItem` (`self.Zone Locations`) `Current Zone Index`) (`|GetArrayItem` (`self.Zone Locations`) `To Action Index`) _alpha)))
    (:`Finished`
      (set `self.Current Action Index` `To Action Index`)
      (`|ExecutionSequence`
        (:`then_0`
          ;;[1 1 1] Call Event On Zone Shrinking Finished
          (`self.Event On Zone Shrinking Finished`))
        (:`then_1`
          ;;[1 1 1] Dont Generate Overlap Events If Radius = 0
          (if (== _radius_2 0.0)
            (set `PrimitiveComponent.bGenerateOverlapEvents` false (`self.SM_Zone`))))))))

(event `Toggle Postprocess Effect`
  (params (Toggle :type Boolean))
  ;[0 0 0] Toggle Postprocess Effect when In/Out Zone
  (if Toggle
    (`|ExecutionSequence`
      (:`then_0`
        (`/Engine/EditorBlueprintResources/StandardMacros.DoOnce` false :!label _label
          (:`Completed`
            (`GameplayStatics.PlaySound2D` (`self.Camera In Zone Sound`) 2.5 1.0 0.0 null null)
            (bind (_direction _weight) (`Timeline|Postprocess Effect` :!label _label_2)
              (:`Update`
                (set `PostProcessComponent.BlendWeight` _weight (`self.OutZonePostprocess`)))))))
      (:`then_1`
        (goto _label_3 :!via `Reset`)))
    (else
      (`|ExecutionSequence`
        (:`then_0`
          (`/Engine/EditorBlueprintResources/StandardMacros.DoOnce` true :!label _label_3
            (:`Completed`
              (`GameplayStatics.PlaySound2D` (`self.Camera Out of Zone Sound`) 2.5 1.0 0.0 null null)
              (goto _label_2 :!via `Reverse`))))
        (:`then_1`
          (goto _label :!via `Reset`))))))

(event `Call Players Zone Status Changed`
  (params (Status :type "/Game/AdvancedBattleRoyaleZone/Blueprint/Enumeration/E_Zone_Status Enum" :default "NewEnumerator0") (`Finished?` :type Boolean) (`Zone Duration` :type "Float (double-precision)"))
  ;[0.3648 0.4375 0.0887] Call Players Event On Zone Status Changed
  (bind _outactors (`GameplayStatics.GetAllActorsOfClass` "/Game/AdvancedBattleRoyaleZone/ThirdPersonBP/Blueprints/ThirdPersonCharacter.ThirdPersonCharacter_C"))
  (for _array_element _outactors
    (`/Game/AdvancedBattleRoyaleZone/Blueprint/BPC_AdvancedBRZone.Event Zone Status Changed` (`/Game/AdvancedBattleRoyaleZone/Blueprint/BFL_BRZone.Get Zone Component` _array_element) Status `Finished?` `Zone Duration`)))

(fn `Generate New Location For Zone`
  (bind _zone_locations (`self.Zone Locations`))
  (bind (_output_x _output_y) (`KismetMathLibrary.BreakVector` (`|GetArrayItem` _zone_locations (`KismetArrayLibrary.Array_LastIndex` _zone_locations))))
  (for (_ _array_index) (`self.Zone Actions`)
    (if (> (`KismetArrayLibrary.Array_Length` (`self.Zone Locations`)) 0)
      (bind ((`Radius_13_BD564BF94CFDF298438BDFABA2539C44` _radius)) (break `/Game/AdvancedBattleRoyaleZone/Blueprint/Structure/S_Zone_Actions` (`|GetArrayItem` (`self.Zone Actions`) (- _array_index 1))))
      (bind ((`Radius_13_BD564BF94CFDF298438BDFABA2539C44` _radius_2)) (break `/Game/AdvancedBattleRoyaleZone/Blueprint/Structure/S_Zone_Actions` (`|GetArrayItem` (`self.Zone Actions`) _array_index)))
      (bind (_returnvalue_x _returnvalue_y) (`KismetMathLibrary.BreakVector` (* (`KismetMathLibrary.GetForwardVector` (`KismetMathLibrary.MakeRotator` 0.0 0.0 (`KismetMathLibrary.RandomFloatInRange` -180.0 180.0))) (select `bool` (> _radius _radius_2) :`true` (* (/ (- _radius _radius_2) 2.0) 100.0)))))
      ;[1 1 1] Add New Location To Array
      (`KismetArrayLibrary.Array_Add` (`self.Zone Locations`) (`KismetMathLibrary.MakeVector` (+ _output_x (* _returnvalue_x (`KismetMathLibrary.RandomFloatInRange` 0.0 1.0))) (+ _output_y (* _returnvalue_y (`KismetMathLibrary.RandomFloatInRange` 0.0 1.0)))))
      (else
        ;[1 1 1] Firs Index Should be always 0,0,0
        (`KismetArrayLibrary.Array_Add` (`self.Zone Locations`)))))
  (return))

(fn `Set Zone Transform`
  (params (Radius :type "Float (double-precision)") (Height :type "Float (double-precision)") (Location :type "Vector Structure"))
  (`SceneComponent.SetRelativeScale3D` (`self.SM_Zone`) (`KismetMathLibrary.MakeVector` Radius Radius Height))
  (if (not (`self.Disable Changing Position`))
    (`SceneComponent.K2_SetRelativeLocation` (`self.SM_Zone`) Location false false)
    (else
      (`SceneComponent.K2_SetRelativeLocation` (`self.SM_Zone`) (0.0 0.0 0.0) false false))))

(fn `UserConstructionScript`
  (bind (_radius _height) (break `/Game/AdvancedBattleRoyaleZone/Blueprint/Structure/S_Zone_Actions` (`|GetArrayItem` (`self.Zone Actions`))))
  (`|ExecutionSequence`
    (:`then_0`
      (if (`KismetArrayLibrary.Array_IsValidIndex` (`self.Zone Actions`))
        (`self.Set Zone Transform` _radius _height)))
    (:`then_1`
      (`self.Set Parameter Collections`)
      (`AudioComponent.SetSound` (`self.Zone_Audio`) (`self.Zone Sound`)))))