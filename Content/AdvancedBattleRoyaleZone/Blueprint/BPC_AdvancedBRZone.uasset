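; Pawn component that handles a player's side of the battle royale zone: outside damage, effects and HUD.
; Authority runs a looping timer that damages the pawn when its XY distance from the BP_Zone center exceeds the radius.
; The local player polls camera or character distance to toggle post-process and fade zone audio.
; Zone status events drive HUD countdown, animations and sounds; separate InZone/OutOfZone events also toggle a damage timer.
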(event `self.ReceiveBeginPlay`
  ;[1 1 1] Begin Play
  (bind _aspawn (cast `Pawn` (`self.GetOwner`)))
  (`|ExecutionSequence`
    (:`then_0`
      ;;[1 0 0] Destroy Component If The Zone Is not Valid (Error Prevention)
      (`/Engine/EditorBlueprintResources/StandardMacros.IsValid` (`self.Get Zone Reference`)
        (:`Is Not Valid`
          (`self.K2_DestroyComponent`))))
    (:`then_1`
      (if (`Actor.HasAuthority` _aspawn)
        (`KismetSystemLibrary.K2_SetTimer` self "Apply Damage Outside Zone" (`/Game/AdvancedBattleRoyaleZone/Blueprint/BP_Zone.Damage Delay` (`self.Get Zone Reference`)) true)))
    (:`then_2`
      (if (`Pawn.IsLocallyControlled` _aspawn)
        (`self.Create Camera Distance Timer`)
        (`self.Create HUD`)))))

(event `Create HUD`
  ;[1 1 1] Create HUD
  (bind _returnvalue (`|CreateWidget` "/Game/AdvancedBattleRoyaleZone/Widget/W_HUD.W_HUD_C"))
  (bind _output_get (set `self.HUD` _returnvalue))
  (`UserWidget.AddToViewport` _output_get 0))

(event `Create Camera Distance Timer`
  ;[0 0 0] Camera Postprocess Effect
  (`KismetSystemLibrary.K2_SetTimerDelegate` (delegate `Zone Postprocess Distance Check`) 0.1 true))

(event `Zone Postprocess Distance Check`
  (bind _zone_reference (`self.Get Zone Reference`))
  (bind _zone_reference_2 (`self.Get Zone Reference`))
  (bind _zone_reference_3 (`self.Get Zone Reference`))
  (bind _zone_reference_4 (`self.Get Zone Reference`))
  (bind _zone_audio (`/Game/AdvancedBattleRoyaleZone/Blueprint/BP_Zone.Zone_Audio` _zone_reference_4))
  (bind _sm_zone (`/Game/AdvancedBattleRoyaleZone/Blueprint/BP_Zone.SM_Zone` _zone_reference))
  (bind _returnvalue_x (`KismetMathLibrary.BreakVector` (`SceneComponent.K2_GetComponentScale` _sm_zone)))
  (bind _returnvalue (/ (* _returnvalue_x 100.0) 2.0))
  (bind _returnvalue_2 (`KismetMathLibrary.VSizeXY` (- (select `/Game/AdvancedBattleRoyaleZone/Blueprint/Enumeration/E_EffectLocation` (`/Game/AdvancedBattleRoyaleZone/Blueprint/BP_Zone.Outside Zone Effect Location` _zone_reference) :`NewEnumerator0` (`PlayerCameraManager.GetCameraLocation` (`GameplayStatics.GetPlayerCameraManager` 0)) :`NewEnumerator1` (`Actor.K2_GetActorLocation` (`self.GetOwner`))) (+ (`SceneComponent.RelativeLocation` _sm_zone) (`Actor.K2_GetActorLocation` _zone_reference)))))
  ;[0 0 0] Camera Postprocess Effect
  (`/Engine/EditorBlueprintResources/StandardMacros.IsValid` (`self.Get Zone Reference`)
    (:`Is Valid`
      (`/Engine/EditorBlueprintResources/StandardMacros.IsValid` (`/Game/AdvancedBattleRoyaleZone/Blueprint/BP_Zone.SM_Zone` (`self.Get Zone Reference`))
        (:`Is Valid`
          ;;[1 1 1] Toggle Postprocess Effect
          (if (> _returnvalue_2 _returnvalue)
            (`/Game/AdvancedBattleRoyaleZone/Blueprint/BP_Zone.Toggle Postprocess Effect` _zone_reference_3 true)
            (`AudioComponent.SetVolumeMultiplier` _zone_audio (`/Game/AdvancedBattleRoyaleZone/Blueprint/BP_Zone.Zone Audio Max Volume` _zone_reference_4))
            (else
              (`/Game/AdvancedBattleRoyaleZone/Blueprint/BP_Zone.Toggle Postprocess Effect` _zone_reference_3 false)
              (`AudioComponent.SetVolumeMultiplier` _zone_audio (`KismetMathLibrary.Lerp` (`/Game/AdvancedBattleRoyaleZone/Blueprint/BP_Zone.Zone Audio Max Volume` (`self.Get Zone Reference`)) 0.0 (`KismetMathLibrary.FClamp` (/ (- (`KismetMathLibrary.Abs` (- _returnvalue_2 _returnvalue)) (`/Game/AdvancedBattleRoyaleZone/Blueprint/BP_Zone.Zone Audio Distance` _zone_reference_2)) (`/Game/AdvancedBattleRoyaleZone/Blueprint/BP_Zone.Zone Audio Fade Distance` _zone_reference_2))))))))))))

(event `In Zone`
  (bind _damage_timer_reference (`self.Damage Timer Reference`))
  ;[0 0.6686 1] Player In Zone
  (if (not (`self.Is In Zone ?`))
    (set `self.Is In Zone ?` true)
    (if (`KismetSystemLibrary.K2_IsValidTimerHandle` _damage_timer_reference)
      (`KismetSystemLibrary.K2_ClearAndInvalidateTimerHandle` _damage_timer_reference))))

(event `Out Of Zone`
  ;[1 0 0] Player Out Of Zone
  (if (`self.Is In Zone ?`)
    (set `self.Is In Zone ?` false)
    (bind _returnvalue (`KismetSystemLibrary.K2_SetTimerDelegate` (delegate `Apply Damage`) (`/Game/AdvancedBattleRoyaleZone/Blueprint/BP_Zone.Damage Delay` (`self.Get Zone Reference`)) true))
    (set `self.Damage Timer Reference` _returnvalue)))

(event `Apply Damage`
  (bind _zone_reference (`self.Get Zone Reference`))
  (bind ((`OutsideDamage_14_D45B34284D3101EAB3A94FB784EB3B69` _outsidedamage)) (break `/Game/AdvancedBattleRoyaleZone/Blueprint/Structure/S_Zone_Actions` (`|GetArrayItem` (`/Game/AdvancedBattleRoyaleZone/Blueprint/BP_Zone.Zone Actions` _zone_reference) (`/Game/AdvancedBattleRoyaleZone/Blueprint/BP_Zone.Current Action Index` _zone_reference))))
  ;[0 0 0] Aply Damage When Player Is Out Of Zone
  ;;[1 1 1] Damaging Player
  (`GameplayStatics.ApplyDamage` (`self.GetOwner`) _outsidedamage null (`self.Get Zone Reference`))
  (`KismetSystemLibrary.PrintString` (`KismetStringLibrary.Concat_StrStr` "[ABRZ] Damage Received - " (`KismetStringLibrary.Conv_DoubleToString` _outsidedamage))))

(event `Create Zone Shrinks In Timer`
  (params (Time :type "Float (double-precision)") (`Zone Status` :type "/Game/AdvancedBattleRoyaleZone/Blueprint/Enumeration/E_Zone_Status Enum" :default "NewEnumerator0"))
  (bind _time_timer (`self.Time Timer`))
  (bind _hud (`self.HUD`))
  ;[0 0 0] Player Time Counter
  ;;[1 1 1] Set Variables
  (set `self.Time` Time)
  (set `self.Actual Zone Status` `Zone Status`)
  ;;[1 1 1] Play Animation and Load Time
  (`/Game/AdvancedBattleRoyaleZone/Widget/W_HUD.Play Popup Animation` _hud)
  (`/Game/AdvancedBattleRoyaleZone/Widget/W_HUD.Load Time` _hud (`self.Time`) (`self.Actual Zone Status`))
  ;;[1 1 1] Create Time Timer
  (if (`KismetSystemLibrary.K2_IsValidTimerHandle` _time_timer)
    (`KismetSystemLibrary.K2_ClearAndInvalidateTimerHandle` _time_timer))
  (bind _returnvalue (`KismetSystemLibrary.K2_SetTimerDelegate` (delegate `Zone Shrinks In Time Update`) 1.0 true))
  (set `self.Time Timer` _returnvalue))

(event `Zone Shrinks In Time Update`
  (bind _hud (`self.HUD`))
  ;[0 0 0] Player Time Counter
  ;;[0.2292 0.2172 0.1165] Time Update Event
  (bind _result (`/Engine/EditorBlueprintResources/StandardMacros.DecrementFloat` (`self.Time`))
    (:`  `
      (if (>= _result 0.0)
        ;;;[1 1 1] Load Time
        (`/Game/AdvancedBattleRoyaleZone/Widget/W_HUD.Load Time` _hud _result (`self.Actual Zone Status`))
        (else
          ;;;[1 1 1] Hide Animation Can Be Played only if Time Appeared
          (`/Game/AdvancedBattleRoyaleZone/Widget/W_HUD.Play Hide Animation` _hud)
          ;;;[1 1 1] Destroy Time Timer
          (`KismetSystemLibrary.K2_ClearAndInvalidateTimerHandle` (`self.Time Timer`)))))))

(event `Event Zone Status Changed`
  (params (`Zone Status` :type "/Game/AdvancedBattleRoyaleZone/Blueprint/Enumeration/E_Zone_Status Enum" :default "NewEnumerator0") (`Finished?` :type Boolean) (Time :type "Float (double-precision)"))
  (bind _zone_reference (`self.Get Zone Reference`))
  ;[0.05208 0.02441 0.02441] Event On Zone Status Changed (Client Event)
  (if `Finished?`
    (switch `/Game/AdvancedBattleRoyaleZone/Blueprint/Enumeration/E_Zone_Status` `Zone Status`
      (:`NewEnumerator1`
        (`GameplayStatics.PlaySound2D` (`/Game/AdvancedBattleRoyaleZone/Blueprint/BP_Zone.Zone Starts Waiting For Shrinking Sound` _zone_reference) 1.0 1.0 0.0 null null)))
    (else
      (`self.Create Zone Shrinks In Timer` (- Time 1.0) `Zone Status`)
      (switch `/Game/AdvancedBattleRoyaleZone/Blueprint/Enumeration/E_Zone_Status` `Zone Status`
        (:`NewEnumerator1`
          (`/Game/AdvancedBattleRoyaleZone/Widget/W_HUD.Play ProgressBar Animation` (`self.HUD`) Time)
          (`GameplayStatics.PlaySound2D` (`/Game/AdvancedBattleRoyaleZone/Blueprint/BP_Zone.Zone Starts Shrinking Sound` _zone_reference) 1.0 1.0 0.0 null null))))))

(fn `Apply Damage Outside Zone`
  (bind _zone_reference (`self.Get Zone Reference`))
  (bind _zone_reference_2 (`self.Get Zone Reference`))
  (bind _sm_zone (`/Game/AdvancedBattleRoyaleZone/Blueprint/BP_Zone.SM_Zone` _zone_reference))
  (bind _returnvalue_x (`KismetMathLibrary.BreakVector` (`SceneComponent.K2_GetComponentScale` _sm_zone)))
  (if (> (`KismetMathLibrary.VSizeXY` (- (`Actor.K2_GetActorLocation` (`self.GetOwner`)) (+ (`SceneComponent.RelativeLocation` _sm_zone) (`Actor.K2_GetActorLocation` _zone_reference)))) (/ (* _returnvalue_x 100.0) 2.0))
    ;[1 1 1] Apply Damage
    (`GameplayStatics.ApplyDamage` (`self.GetOwner`) (`.OutsideDamage_14_D45B34284D3101EAB3A94FB784EB3B69` (break `/Game/AdvancedBattleRoyaleZone/Blueprint/Structure/S_Zone_Actions` (`|GetArrayItem` (`/Game/AdvancedBattleRoyaleZone/Blueprint/BP_Zone.Zone Actions` _zone_reference_2) (`/Game/AdvancedBattleRoyaleZone/Blueprint/BP_Zone.Current Action Index` _zone_reference_2)))) null (`self.Get Zone Reference`))
    (`KismetSystemLibrary.PrintString` "ABRZ: Player Damaged" true true (struct :`R` 1.0 :`A` 1.0))))

(fn `Get Zone Reference`
  (returns (`Zone Reference` :type "/Game/AdvancedBattleRoyaleZone/Blueprint/BP_Zone Object Reference"))
  (bind _outactors (`GameplayStatics.GetAllActorsOfClass` "/Game/AdvancedBattleRoyaleZone/Blueprint/BP_Zone.BP_Zone_C"))
  (return (`|GetArrayItem` _outactors)))